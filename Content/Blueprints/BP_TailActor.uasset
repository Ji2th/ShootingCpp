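; BP_TailActor is an Actor sketched to follow a target at a set speed, but none of its logic currently runs.
; Disconnected nodes would default a null target to player pawn 0, as a comment on BeginPlay intends.
; A second disconnected chain would move it along the normalized direction to the target, scaled by speed and delta time, without sweep.
; BeginPlay, Tick and the construction script are all empty.
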(event EventBeginPlay
  ;[1 1 1] 태어날 때 target이 Null이라면 target을 주인공으로 하고싶다.
)

(event Collision|EventActorBeginOverlap
  (params (OtherActor :type Actor%20Object%20Reference)))

(event EventTick
  (params (DeltaSeconds :type Float%20%28single-precision%29))
  ;[1 1 1] P = P0 + v(방향 * speed) * t
)

(fn ConstructionScript)