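; BP_BulletActor is a projectile that flies straight ahead and destroys enemies it hits.
; Each Tick moves it along its forward vector by Speed scaled by delta time, setting the location directly without sweeping.
; On overlap with a BP_EnemyActor, it spawns an explosion particle at the enemy's location, then destroys both the enemy and itself.
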(event EventBeginPlay)

(event Collision|EventActorBeginOverlap
  (params (OtherActor :type Actor%20Object%20Reference))
  ;[1 1 1] Bullet이 Enemy와 부딪혔다!!! VFX만들고 너죽고 나죽자
  (bind _asbp_enemy_actor (Utilities|Casting|CastToBP_EnemyActor OtherActor))
  (Effects|SpawnEmitteratLocation "/Game/StarterContent/Particles/P_Explosion.P_Explosion" (Transformation|GetActorLocation _asbp_enemy_actor))
  (Actor|DestroyActor _asbp_enemy_actor)
  (Actor|DestroyActor))

(event EventTick
  (params (DeltaSeconds :type Float%20%28single-precision%29))
  ;[1 1 1] P = P0 + v(방향 * speed) * t
  (Transformation|SetActorLocation (+ (* (* (Transformation|GetActorForwardVector) (Variables|Default|Getspeed)) DeltaSeconds) (Transformation|GetActorLocation)) false false))

(fn ConstructionScript)