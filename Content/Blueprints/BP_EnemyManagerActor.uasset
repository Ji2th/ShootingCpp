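; BP_EnemyManagerActor is an enemy spawner that periodically creates BP_EnemyActor instances at its Arrow component's location and rotation.
; Tick accumulates elapsed time and, once it exceeds CreateTime while player pawn 0 is valid, calls MakeEnemy and resets the counter.
; MakeEnemy always spawns regardless of collision.
; Unconnected Delay, timer-by-function-name and timer-by-event variants remain in the graph but never run.
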(event Custom|Event%20MakeEnemy
  ;[1 1 1] 이벤트를 타이머에 등록하기
  (CallFunction|MakeEnemy))

(event EventBeginPlay)

(event Collision|EventActorBeginOverlap
  (params (OtherActor :type Actor%20Object%20Reference)))

(event EventTick
  (params (DeltaSeconds :type Float%20%28single-precision%29))
  ;[1 1 1] 1. 시간이 흐르다가
  ; 2. 만약 현재시간이 생성시간을 초과하면
  ; 3. 적공장에서 적을 생성해서 화살표 위치에 배치하고싶다.
  ; 4. 현재시간을 0으로 초기화 하고싶다.
  (bind _output_get (Variables|Default|SetcurrentTime (+ DeltaSeconds (Variables|Default|GetcurrentTime))))
  (if (> _output_get (Variables|Default|GetcreateTime))
    (Utilities|IsValid (Game|Player|GetPlayerPawn 0)
      (:Is%20Valid
        (CallFunction|MakeEnemy)
        (Variables|Default|SetcurrentTime 0.0)))))

(fn ConstructionScript)

(fn MakeEnemy
  (bind _arrow (Variables|Default|GetArrow))
  (bind _returnvalue (Transformation|GetWorldTransform _arrow))
  (Game|SpawnActorfromClass "/Game/Blueprints/BP_EnemyActor.BP_EnemyActor_C" (Math|Transform|MakeTransform (.location _returnvalue) (.rotation _returnvalue) "1,1,1") "AlwaysSpawn" 0 0))